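; BP_FollowButton is an actor in the lobby click folder that floats along with the VR player.
; On BeginPlay it caches player pawn 0 as a BP_VRPawn.
; Each Tick it eases toward the pawn's Scene component with VInterpTo and snaps its rotation to the look-at direction from that component to the pawn's location, so it faces the player.
; The graph holds no click handling.
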(event EventBeginPlay
  (bind _asbp_vrpawn (Utilities|Casting|CastToBP_VRPawn (Game|Player|GetPlayerPawn 0)))
  (Variables|Default|SetAs%20VRPawn _asbp_vrpawn))

(event Collision|EventActorBeginOverlap
  (params (OtherActor :type Actor%20Object%20Reference)))

(event EventTick
  (params (DeltaSeconds :type Float%20%28single-precision%29))
  (bind _as_vrpawn (Variables|Default|GetAs%20VRPawn))
  (bind _scene (Variables|/Game/_Project/Blueprints/BP_VRPawn.BP_VRPawn_C|GetScene _as_vrpawn))
  (bind _returnvalue (Transformation|GetWorldLocation _scene))
  (Utilities|IsValid (Variables|Default|GetAs%20VRPawn)
    (:Is%20Valid
      (Transformation|SetActorLocationAndRotation (Math|Interpolation|VInterpTo (Transformation|GetActorLocation) _returnvalue DeltaSeconds 7.0) (Math|Rotator|FindLookatRotation _returnvalue (Transformation|GetActorLocation _as_vrpawn))))))

(fn ConstructionScript)