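; BP_Loading is a VR loading screen actor that shows a randomly chosen Korean message about travelling to Dokdo.
; On BeginPlay it attaches to the BP_VRPawn's CameraOrigin and sets a fixed relative offset in front of and slightly below it.
; It then gets the WBP_Loading widget from its Loading component and writes one of five hard-coded messages into LoadingMain.
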(event EventBeginPlay
  (Transformation|AttachComponentToComponent (Variables|/Game/_Project/Blueprints/BP_VRPawn.BP_VRPawn_C|GetCameraOrigin (.AsBP%20VRPawn (Utilities|Casting|CastToBP_VRPawn (Game|Player|GetPlayerPawn 0)))) "None" "KeepRelative" "KeepRelative" "KeepRelative" true)
  (Transformation|SetActorRelativeTransform (Math|Transform|MakeTransform "1000.000000,0.000000,-50.000000" "0, 0, 0" "1.000000,1.000000,1.000000") false false)
  (bind _aswbp_loading (Utilities|Casting|CastToWBP_Loading (UserInterface|GetWidget (Variables|Default|GetLoading))))
  (switch int (Math|Random|RandomIntegerinRange 0 4)
    (:0
      (Variables|Default|SetSetLoadingMain "독도가 가까워지고 있습니다!"))
    (:1
      (Variables|Default|SetSetLoadingMain "동해 위 독도로 항해 중!"))
    (:2
      (Variables|Default|SetSetLoadingMain "파도 소리와 함께 독도로!"))
    (:3
      (Variables|Default|SetSetLoadingMain "우리 땅, 독도로 향합니다."))
    (:4
      (Variables|Default|SetSetLoadingMain "독도가 기다리고 있습니다.")))
  (Variables|/Game/_Project/Blueprints/WBP_Loading.WBP_Loading_C|SetLoadingMain _aswbp_loading (Variables|Default|GetSetLoadingMain)))

(fn ConstructionScript)