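; BP_MasterButton is a lobby button actor that shows its label through a WBP_Buttons widget component.
; On BeginPlay it casts the widget and passes TextName to it as the displayed text.
; A Rotate event smoothly yaws the actor toward a VR pawn reference, but the pawn lookup and looping timer meant to drive it are disconnected, so the button does not turn.
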(event Custom|Rotate
  (Transformation|SetActorRotation (Math|Rotator|MakeRotator 0.0 0.0 (.yaw (Math|Interpolation|RInterpTo (Transformation|GetActorRotation) (Math|Rotator|FindLookatRotation (Transformation|GetActorLocation) (Transformation|GetActorLocation (Variables|Default|GetBP_VRPawn))) (Utilities|Time|GetWorldDeltaSeconds) 2.0)))))

(event EventBeginPlay
  (bind _aswbp_buttons (Utilities|Casting|CastToWBP_Buttons (UserInterface|GetUserWidgetObject (Variables|Default|GetButton))))
  (Variables|/Game/_Project/Blueprints/_Lobby/WBP_Buttons.WBP_Buttons_C|SetGet%20Text _aswbp_buttons (Utilities|Text|ToText(String) (Variables|Default|GetText%20Name))))

(event Collision|EventActorBeginOverlap
  (params (OtherActor :type Actor%20Object%20Reference)))

(event EventTick
  (params (DeltaSeconds :type Float%20%28single-precision%29)))

(fn ConstructionScript)