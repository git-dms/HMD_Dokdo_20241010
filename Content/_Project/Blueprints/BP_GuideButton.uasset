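; BP_GuideButton is an actor that shows a named guide label through a WBP_GuideButton widget component.
; BeginPlay passes its TextName to the widget, and Tick smoothly turns the actor on yaw to face the player pawn.
; LobbyClear activates or deactivates the widget by its IsMainMenu flag, playing or reversing a timeline that scales it up or down from its original scale.
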(event Custom|LobbyClear
  (params (IsMainMenu :type Boolean))
  (bind _guidebutton (Variables|Default|GetGuideButton))
  ;[0 0 0] Lobby Clear
  (if IsMainMenu
    (Components|Activation|Deactivate _guidebutton)
    (bind _alpha (Timeline|Timeline Reverse)
      (:Update
        (Transformation|SetRelativeScale3D (Variables|Default|GetGuideButton) (Math|Conversions|ToVector(Float) (* _alpha (Variables|Default|GetWidgetRelativeScaleOriginal))))))
    (else
      (Components|Activation|Activate _guidebutton false)
      (Timeline|Timeline Play))))

(event EventBeginPlay
  ;[0 0 0] BeginPlay
  (bind _aswbp_guide_button (Utilities|Casting|CastToWBP_GuideButton (UserInterface|GetUserWidgetObject (Variables|Default|GetGuideButton))))
  (Variables|/Game/_Project/Blueprints/WBP_GuideButton.WBP_GuideButton_C|SetGet%20Text _aswbp_guide_button (Utilities|Text|ToText(String) (Variables|Default|GetText%20Name))))

(event EventTick
  (params (DeltaSeconds :type Float%20%28single-precision%29))
  ;[0 0 0] Set Rotation Towards Player
  (Transformation|SetActorRotation (Math|Rotator|MakeRotator 0.0 0.0 (.yaw (Math|Interpolation|RInterpTo (Transformation|GetActorRotation) (Math|Rotator|FindLookatRotation (Transformation|GetActorLocation) (Transformation|GetActorLocation (Game|Player|GetPlayerPawn 0))) (Utilities|Time|GetWorldDeltaSeconds) 5.0)))))

(fn ConstructionScript)