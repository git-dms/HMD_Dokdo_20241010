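; VR video button actor that attaches to the player pawn's CameraOrigin and plays a video on a mesh detached at the pawn's location.
; PlayVideo selects a source by pawn Index (all four cases use Centipede), shows the mesh and opens the media player; ExitVideo reverses this.
; Timelines scale Play and Exit widgets in and out, both using Play's stored scale.
; The right shoot input drives widget clicks.
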(event Custom|PlayVideo
  (bind _mediaplayer (Variables|Default|GetMediaPlayer))
  (CallFunction|ClosePlayButton false)
  (Rendering|SetVisibility (Variables|Default|GetStaticMesh) true false)
  (Rendering|SetVisibility (Variables|Default|GetExit) true false)
  (bind _asbp_vrpawn (Utilities|Casting|CastToBP_VRPawn (Game|Player|GetPlayerPawn 0)))
  (switch int (Variables|/Game/_Project/Blueprints/BP_VRPawn.BP_VRPawn_C|GetIndex _asbp_vrpawn)
    (:0
      (Variables|Default|SetMedia%20Source "/Game/_Project/Movie/Centipede.Centipede"))
    (:1
      (Variables|Default|SetMedia%20Source "/Game/_Project/Movie/Centipede.Centipede"))
    (:2
      (Variables|Default|SetMedia%20Source "/Game/_Project/Movie/Centipede.Centipede"))
    (:3
      (Variables|Default|SetMedia%20Source "/Game/_Project/Movie/Centipede.Centipede")))
  (Class|MediaPlayer|OpenSourceLatent _mediaplayer (Variables|Default|GetMedia%20Source))
  (Media|MediaPlayer|Play _mediaplayer :!class /Script/MediaAssets.MediaPlayer)
  (CallFunction|OpenExitButton))

(event Custom|ExitVideo
  (Media|MediaPlayer|Close (Variables|Default|GetMediaPlayer) :!class /Script/MediaAssets.MediaPlayer)
  (Rendering|SetVisibility (Variables|Default|GetStaticMesh) false false)
  (CallFunction|CloseExitButton)
  (CallFunction|OpenPlayButton))

(event Custom|CloseExitButton
  (bind _exit (Variables|Default|GetExit))
  (bind (_direction _alpha) (Timeline|Timeline_0 Reverse)
    (:Update
      (Transformation|SetRelativeScale3D _exit (Math|Conversions|ToVector(Float) (* _alpha (Variables|Default|GetPlayWidgetRelativeScaleOriginal)))))
    (:Finished
      (if (Utilities|Enum|Equal(Enum) _direction "Backward")
        (Components|Activation|Deactivate _exit)))))

(event Custom|OpenExitButton
  (bind _exit (Variables|Default|GetExit))
  (bind _exit_2 (Variables|Default|GetExit))
  (Components|Activation|Activate _exit false)
  (Variables|Default|SetExitWidgetRelativeScaleOriginal (.x (Variables|/Script/Engine.SceneComponent|GetRelativeScale3D _exit)))
  (bind (_direction _alpha) (Timeline|Timeline_0 Play)
    (:Update
      (Transformation|SetRelativeScale3D _exit_2 (Math|Conversions|ToVector(Float) (* _alpha (Variables|Default|GetPlayWidgetRelativeScaleOriginal)))))
    (:Finished
      (if (Utilities|Enum|Equal(Enum) _direction "Backward")
        (Components|Activation|Deactivate _exit_2)))))

(event Custom|ClosePlayButton
  (params (DestroyEverything :type Boolean))
  (bind (_direction _alpha) (Timeline|Timeline Reverse)
    (:Update
      (Transformation|SetRelativeScale3D (Variables|Default|GetPlay) (Math|Conversions|ToVector(Float) (* _alpha (Variables|Default|GetPlayWidgetRelativeScaleOriginal)))))
    (:Finished
      (if (Utilities|Enum|Equal(Enum) _direction "Backward")
        (if DestroyEverything
          (Actor|DestroyActor)
          (else
            (Components|Activation|Deactivate (Variables|Default|GetPlay))))))))

(event Custom|OpenPlayButton
  (bind _play (Variables|Default|GetPlay))
  (Components|Activation|Activate _play false)
  (Variables|Default|SetPlayWidgetRelativeScaleOriginal (.x (Variables|/Script/Engine.SceneComponent|GetRelativeScale3D _play))) ; Set the original relative scale
  (bind (_direction _alpha) (Timeline|Timeline Play)
    (:Update
      (Transformation|SetRelativeScale3D (Variables|Default|GetPlay) (Math|Conversions|ToVector(Float) (* _alpha (Variables|Default|GetPlayWidgetRelativeScaleOriginal)))))
    (:Finished
      (if (Utilities|Enum|Equal(Enum) _direction "Backward")
        (if (stale Custom|ClosePlayButton DestroyEverything)
          (Actor|DestroyActor)
          (else
            (Components|Activation|Deactivate (Variables|Default|GetPlay))))))))

(event Input|EnhancedActionEvents|EnhancedInputActionIA_Shoot_Right
  (params (ActionValue :type Boolean) (ElapsedSeconds :type Float%20%28double-precision%29) (TriggeredSeconds :type Float%20%28double-precision%29) (InputAction :type Input%20Action%20Object%20Reference :default "/Game/VRTemplate/Input/Actions/IA_Shoot_Right.IA_Shoot_Right"))
  (bind _widget_interaction_component (Variables|Default|GetWidget%20Interaction%20Component))
  (:Triggered
    (Class|WidgetInteractionComponent|PressPointerKey _widget_interaction_component "LeftMouseButton"))
  (:Completed
    (Class|WidgetInteractionComponent|ReleasePointerKey _widget_interaction_component "LeftMouseButton")))

(event EventBeginPlay
  (bind _returnvalue (Game|Player|GetPlayerPawn 0))
  (bind _staticmesh (Variables|Default|GetStaticMesh))
  (bind _asbp_vrpawn (Utilities|Casting|CastToBP_VRPawn _returnvalue))
  (Transformation|AttachComponentToComponent (Variables|/Game/_Project/Blueprints/BP_VRPawn.BP_VRPawn_C|GetCameraOrigin _asbp_vrpawn) "None" "KeepRelative" "KeepRelative" "KeepRelative" true)
  (Transformation|SetActorRelativeTransform (Math|Transform|MakeTransform "0, 0, 0" "0.000000,180.000000,0.000000" "1.000000,1.000000,1.000000") false false)
  (Transformation|DetachFromComponent _staticmesh "KeepRelative" "KeepRelative" "KeepRelative" true)
  (Transformation|SetWorldLocation _staticmesh (Transformation|GetActorLocation _asbp_vrpawn) false true))

(event Collision|EventActorBeginOverlap
  (params (OtherActor :type Actor%20Object%20Reference)))

(event EventTick
  (params (DeltaSeconds :type Float%20%28single-precision%29)))

(fn ConstructionScript)