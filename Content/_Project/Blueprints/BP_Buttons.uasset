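; BP_Buttons is a world actor acting as a touchable button, with a widget component that shows its label.
; On BeginPlay it casts the widget to WBP_Buttons, caches it and passes in the actor's ButtonName.
; Overlapping its Box component prints the button's name with a "Button Touch" message to the screen, with no further action wired.
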(event OnComponentBeginOverlap(Box)
  (params (OverlappedComponent :type Primitive%20Component%20Object%20Reference) (OtherActor :type Actor%20Object%20Reference) (OtherComp :type Primitive%20Component%20Object%20Reference) (OtherBodyIndex :type Integer) (bFromSweep :type Boolean) (SweepResult :type Hit%20Result%20Structure%20%28by%20ref%29))
  (Development|PrintString (Utilities|String|Append (Utilities|String|ToString(Object) (Variables|/Game/_Project/Blueprints/WBP_Buttons.WBP_Buttons_C|GetButtonName (Variables|Default|GetAs%20WBP%20Buttons))) ": Button Touch")))

(event EventBeginPlay
  (bind _aswbp_buttons (Utilities|Casting|CastToWBP_Buttons (UserInterface|GetUserWidgetObject (Variables|Default|GetWidget))))
  (bind _output_get (Variables|Default|SetAs%20WBP%20Buttons _aswbp_buttons))
  (Default|SetButtonName _output_get (Variables|Default|GetButton%20Name)))

(event Collision|EventActorBeginOverlap
  (params (OtherActor :type Actor%20Object%20Reference)))

(event EventTick
  (params (DeltaSeconds :type Float%20%28single-precision%29)))

(fn ConstructionScript)